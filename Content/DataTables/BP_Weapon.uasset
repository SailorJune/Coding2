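; BP_Weapon is a weapon actor that shows its type, element and damage range on text components.
; On BeginPlay it registers itself in the game mode's LevelSave list of spawned weapons.
; SpawnWeapon picks a random DT_Weapons row and spawns another BP_Weapon at its own body's location with that row's type, element and base damage.
; RandomizeValues then rolls the new weapon's damage range and refreshes its text.
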(event Custom|SpawnWeapon
  (bind _outrownames (DataTable|GetDataTableRowNames "/Game/DataTables/DT_Weapons.DT_Weapons"))
  (bind _returnvalue (Utilities|GetDataTableRow "/Game/DataTables/DT_Weapons.DT_Weapons" (.OutItem (Utilities|Array|Random _outrownames)))
    (:then
      (bind _returnvalue_2 (Game|SpawnActorfromClass "BP_Weapon_C" (Math|Transform|MakeTransform (Transformation|GetWorldLocation (Variables|Default|GetWeaponBody)) "0, 0, 0" "1.000000,1.000000,1.000000") "Undefined" "MultiplyWithRoot" 0 0))
      (Variables|BP_Weapon_C|SetWeaponType _returnvalue_2 (.weapontype _returnvalue))
      (Variables|BP_Weapon_C|SetElementalType _returnvalue_2 (.elementaltype _returnvalue))
      (Variables|BP_Weapon_C|SetMinDamage _returnvalue_2 (.basedamage _returnvalue))
      (CallFunction|RandomizeValues _returnvalue_2))))

(event Custom|Randomize%20Values
  (bind _output_get (Variables|Default|SetMinDamage (+ (Variables|Default|GetMinDamage) (Math|Random|RandomInteger 2))))
  (Variables|Default|SetMaxDamage (+ _output_get (Math|Random|RandomIntegerinRange 1 4)))
  (CallFunction|UpdateText))

(event Custom|UpdateText
  (Rendering|Components|TextRender|SetText (Variables|Default|GetTextWeaponType) (Utilities|Text|ToText(String) (Utilities|String|EnumtoString (Variables|Default|GetWeaponType))))
  (Rendering|Components|TextRender|SetText (Variables|Default|GetTextElemType) (Utilities|Text|ToText(String) (Utilities|String|EnumtoString (Variables|Default|GetElementalType))))
  (Rendering|Components|TextRender|SetText (Variables|Default|GetTextDmg) (Utilities|Text|ToText(String) (Utilities|String|Append (Utilities|String|ToString(Integer) (Variables|Default|GetMinDamage)) "-" (Utilities|String|ToString(Integer) (Variables|Default|GetMaxDamage))))))

(event EventBeginPlay
  (bind _asgm_coding_2for_real (Utilities|Casting|CastToGM_Coding2ForReal (Game|GetGameMode)))
  (Utilities|Array|AddUnique (Variables|/Game/Blueprints/NewSaves/SG_LevelSave.SG_LevelSave_C|GetSpawnedWeapons (Variables|/Game/Blueprints/GM_Coding2ForReal.GM_Coding2ForReal_C|GetLevel%20Save _asgm_coding_2for_real)) self))

(fn ConstructionScript)