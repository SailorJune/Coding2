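; BP_ToyDoor is a toy door that starts moving by chance and can be held by a HoldDoor event.
; A looping timer with a randomized interval rolls a 50% chance to play a timeline sliding the actor along Y while counting DoorTime.
; HoldDoor resets that count, plays a sound, restarts the timer and briefly flags DoorShut so the roll can stop the timeline.
; Box overlap toggles the W_ToyDoor widget and InRange.
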(event OnComponentBeginOverlap(Box)
  (params (OverlappedComponent :type Primitive%20Component%20Object%20Reference) (OtherActor :type Actor%20Object%20Reference) (OtherComp :type Primitive%20Component%20Object%20Reference) (OtherBodyIndex :type Integer) (bFromSweep :type Boolean) (SweepResult :type Hit%20Result%20Structure%20%28by%20ref%29))
  (Utilities|Casting|CastToBP_ThirdPersonCharacter OtherActor)
  (bind _returnvalue (UserInterface|CreateWidget "/Game/Blueprints/Toy/W_ToyDoor.W_ToyDoor_C"))
  (UserInterface|Viewport|AddtoViewport _returnvalue 0)
  (Variables|Default|SetInRange? true)
  (if (Variables|Default|GetInRange?)
    (Development|PrintString "You're close")
    (else
      (Development|PrintString "You're not close"))))

(event OnComponentEndOverlap(Box)
  (params (OverlappedComponent :type Primitive%20Component%20Object%20Reference) (OtherActor :type Actor%20Object%20Reference) (OtherComp :type Primitive%20Component%20Object%20Reference) (OtherBodyIndex :type Integer))
  (Widget|RemovefromParent (stale OnComponentBeginOverlap(Box) _returnvalue))
  (Variables|Default|SetInRange? false)
  (Development|PrintString "you're far"))

(event Custom|Hold%20Door
  (Variables|Default|SetDoorShut true)
  (Variables|Default|SetDoorTime 0)
  (Audio|PlaySoundatLocation "/Game/Blueprints/Toy/Recording__2_.Recording__2_" (Transformation|GetActorLocation) "0, 0, 0" 1.0 1.0 0.0 0 0 0 0)
  (CallFunction|Timer)
  (CallFunction|ShimmyShimmyYO)
  (Variables|Default|SetDoorShut false))

(event Custom|ShimmyShimmyYO
  (bind _er (Variables|Default|Geter))
  (bind _returnvalue (Transformation|GetWorldLocation _er))
  (Utilities|FlowControl|Sequence
    (:then_0
      (goto _label Open))
    (:then_1
      (Utilities|FlowControl|Gate true :!label _label
        (:Exit
          (if (Math|Random|RandomBoolwithWeight 0.5)
            (if (Variables|Default|GetDoorShut)
              (bind _newtrack_0 (Timeline|Timeline Stop)
                (:Update
                  (Transformation|SetActorLocation (Math|Vector|MakeVector (.x _returnvalue) (+ (.y _returnvalue) _newtrack_0) (.z _returnvalue)) false false)
                  (bind _output_get (Variables|Default|SetDoorTime (+ (Variables|Default|GetDoorTime) 1)))
                  (if (>= _output_get 1000)
                    _)))
              (else
                (Timeline|Timeline Play)))
            (else
              (goto _label))))))))

(event Custom|Timer
  (Utilities|Time|SetTimerbyEvent (delegate Custom|ShimmyShimmyYO) (Math|Random|RandomFloatinRange (Math|Random|RandomFloatinRange 1.0 5.0) (Math|Random|RandomFloatinRange 5.0 1e+01)) true))

(event EventBeginPlay
  (CallFunction|Timer))

(fn ConstructionScript)