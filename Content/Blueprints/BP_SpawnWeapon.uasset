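; BP_SpawnWeapon is a trigger actor that spawns a random weapon whenever the third-person character begins overlapping its sphere.
; It picks a random row from the DD_Weapons data table and spawns a BP_Weapon at the sphere's transform.
; The row's weapon type, element and base damage (as minimum damage) are copied onto the weapon, which then randomizes its values.
; Disconnected text-setting nodes for those stats never run.
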(event OnComponentBeginOverlap(Sphere1)
  (params (OverlappedComponent :type Primitive%20Component%20Object%20Reference) (OtherActor :type Actor%20Object%20Reference) (OtherComp :type Primitive%20Component%20Object%20Reference) (OtherBodyIndex :type Integer) (bFromSweep :type Boolean) (SweepResult :type Hit%20Result%20Structure%20%28by%20ref%29))
  (Utilities|Casting|CastToBP_ThirdPersonCharacter OtherActor)
  (CallFunction|SpawnWeapon))

(event Custom|spawn%20weapon
  (bind _outrownames (DataTable|GetDataTableRowNames "/Game/DataTables/DD_Weapons.DD_Weapons"))
  (bind _returnvalue (Utilities|GetDataTableRow "/Game/DataTables/DD_Weapons.DD_Weapons" (.OutItem (Utilities|Array|Random _outrownames)))
    (:then
      (bind _returnvalue_2 (Game|SpawnActorfromClass "/Game/Blueprints/BP_Weapon.BP_Weapon_C" (Transformation|GetWorldTransform (Variables|Default|GetSphere1)) "Undefined" "MultiplyWithRoot" 0 0))
      (Variables|/Game/Blueprints/BP_Weapon.BP_Weapon_C|SetWpnType _returnvalue_2 (.weapontype _returnvalue))
      (Variables|/Game/Blueprints/BP_Weapon.BP_Weapon_C|SetElmType _returnvalue_2 (.elementaltype _returnvalue))
      (Variables|/Game/Blueprints/BP_Weapon.BP_Weapon_C|SetMinDmg _returnvalue_2 (.basedamage _returnvalue))
      (Default|RandomizeValues _returnvalue_2))))

(fn ConstructionScript)