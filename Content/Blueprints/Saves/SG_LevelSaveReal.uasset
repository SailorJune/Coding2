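; SG_LevelSaveReal is a level save asset that restores which coins are collected and which doors are open.
; It keeps actor references in the CollectedCoins and OpenedDoors arrays, with one load function for each.
; Each function loops over its array, skips invalid references and calls LoadCollectedState on coins or DoorOpened on doors, so each actor applies its own state.
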(fn LoadCollectedCoins
  (if (> (Utilities|Array|Length (Variables|Default|GetCollectedCoins)) 0)
    (for _array_element (Variables|Default|GetCollectedCoins)
      (Utilities|IsValid _array_element
        (:Is%20Valid
          (Default|LoadCollectedState _array_element))))))

(fn LoadCollectedDoors
  (bind _openeddoors (Variables|Default|GetOpenedDoors))
  (if (> (Utilities|Array|Length _openeddoors) 0)
    (for _array_element _openeddoors
      (Utilities|IsValid _array_element
        (:Is%20Valid
          (Default|DoorOpened _array_element))))))