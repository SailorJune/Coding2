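; Game mode that handles per-level save and load of checkpoints, collected coins and door state.
; BeginPlay loads the SG_LevelSaveReal slot named after the current level, or creates a new save object if none exists.
; Loading restores coins, an opened door and the player's transform, skipping the transform when its location is zero.
; Checkpoint stores the player transform and saves, while FinishedLevel clears it and saves.
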(event Custom|SaveGame
  (bind _returnvalue (Game|GetCurrentLevelName true))
  (SaveGame|SaveGametoSlot (Variables|Default|GetLevelSave!) _returnvalue)
  (if true
    (Development|PrintString "Good (Saved)")
    (else
      (Development|PrintString "Bad (Couldn't Save)"))))

(event EventBeginPlay
  (Development|PrintString "Its fucking working my guy" true true "(R=1.000000,G=0.000000,B=0.100863,A=1.000000)" 2e+01)
  (bind _returnvalue (Game|GetCurrentLevelName true))
  (bind _returnvalue_2 (SaveGame|DoesSaveGameExist _returnvalue))
  (if _returnvalue_2
    (bind _returnvalue_3 (SaveGame|LoadGamefromSlot _returnvalue))
    (bind _assg_level_save_real (Utilities|Casting|CastToSG_LevelSaveReal _returnvalue_3))
    (bind _output_get (Variables|Default|SetLevelSave! _assg_level_save_real))
    (Default|LoadCollectedCoins _output_get)
    (if (Variables|/Game/Blueprints/Saves/SG_LevelSaveReal.SG_LevelSaveReal_C|GetDoor%20Open _assg_level_save_real)
      (Default|DoorOpened (Variables|/Game/Blueprints/Saves/SG_LevelSaveReal.SG_LevelSaveReal_C|GetDoor (Variables|Default|GetLevelSave!))))
    (if (not (Class|KismetMathLibrary|EqualExactlyVectorVector (.location (Variables|/Game/Blueprints/Saves/SG_LevelSaveReal.SG_LevelSaveReal_C|GetPlayerTransform (Variables|Default|GetLevelSave!))) "0, 0, 0"))
      (Transformation|SetWorldTransform (Variables|/Script/Engine.Character|GetCapsuleComponent (Game|GetPlayerCharacter 0)) (Variables|/Game/Blueprints/Saves/SG_LevelSaveReal.SG_LevelSaveReal_C|GetPlayerTransform (Variables|Default|GetLevelSave!)) false false))
    (else
      (bind _returnvalue_4 (SaveGame|CreateSaveGameObject "/Game/Blueprints/Saves/SG_LevelSaveReal.SG_LevelSaveReal_C"))
      (Variables|Default|SetLevelSave! _returnvalue_4))))

(fn ConstructionScript)

(fn Checkpoint
  (params (Player%20Transform :type Transform))
  (Variables|/Game/Blueprints/Saves/SG_LevelSaveReal.SG_LevelSaveReal_C|SetPlayerTransform (Variables|Default|GetLevelSave!) Player%20Transform)
  (CallFunction|SaveGame))

(fn FinishedLevel
  (Variables|/Game/Blueprints/Saves/SG_LevelSaveReal.SG_LevelSaveReal_C|SetPlayerTransform (Variables|Default|GetLevelSave!) "")
  (CallFunction|SaveGame))