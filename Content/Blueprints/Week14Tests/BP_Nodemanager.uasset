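; BP_Nodemanager is a test manager actor that grows an endless random chain of BP_Node actors.
; On BeginPlay it spawns an indexed node at its own location, then SpawnNewNode re-calls itself every half second, placing each node randomly in a box around the last.
; Each new node's NextNode and PrevNode both point to the previous node, despite comments intending a two-way link.
; DrawPath is an empty stub for spacebar-triggered link creation.
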(event Custom|SpawnNewNode
  (bind _nodeindex (Variables|Default|GetNodeIndex))
  (Development|PrintString "Spawning a new node!!")
  (bind _returnvalue (Game|SpawnActorfromClass "/Game/Blueprints/Week14Tests/BP_Node.BP_Node_C" (Math|Transform|MakeTransform (Math|Random|RandomPointinBoundingBox (Transformation|GetActorLocation (Variables|Default|GetLastNode)) "500.000000,500.000000,500.000000") "0, 0, 0" "1.000000,1.000000,1.000000") "Undefined" "MultiplyWithRoot" 0 0))
  (Variables|/Game/Blueprints/Week14Tests/BP_Node.BP_Node_C|SetIndex _returnvalue _nodeindex)
  (Math|Integer|IncrementInt _nodeindex
    (:%20%20
      (Variables|/Game/Blueprints/Week14Tests/BP_Node.BP_Node_C|SetNextNode _returnvalue (Variables|Default|GetLastNode)) ; set the "next node" on the first node
      (Variables|/Game/Blueprints/Week14Tests/BP_Node.BP_Node_C|SetPrevNode _returnvalue (Variables|Default|GetLastNode)) ; Set the "previous node" on this new node.
      (Variables|Default|SetLastNode _returnvalue)
      (Utilities|FlowControl|Delay 0.5)
      (CallFunction|SpawnNewNode))))

(event Custom|Draw%20Path)

(event EventBeginPlay
  (bind _nodeindex (Variables|Default|GetNodeIndex))
  (bind _returnvalue (Game|SpawnActorfromClass "/Game/Blueprints/Week14Tests/BP_Node.BP_Node_C" (Math|Transform|MakeTransform (Transformation|GetActorLocation) "0, 0, 0" "1.000000,1.000000,1.000000") "Undefined" "MultiplyWithRoot" 0 0))
  (Variables|Default|SetLastNode _returnvalue)
  (Variables|/Game/Blueprints/Week14Tests/BP_Node.BP_Node_C|SetIndex _returnvalue _nodeindex)
  (Math|Integer|IncrementInt _nodeindex
    (:%20%20
      (CallFunction|SpawnNewNode))))

(fn ConstructionScript)