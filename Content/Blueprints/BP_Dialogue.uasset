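; Dialogue actor that shows a prompt when the player character enters its box and displays dialogue on E press.
; BeginPlay creates the prompt and dialogue widgets, which the overlap and key events add to the viewport.
; Each press reads the next DT_Dialogue row by index, setting the text and an emotion-matched portrait material.
; The E event has no overlap check, and the prompt is never removed.
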(event OnComponentBeginOverlap(Box)
  (params (OverlappedComponent :type Primitive%20Component%20Object%20Reference) (OtherActor :type Actor%20Object%20Reference) (OtherComp :type Primitive%20Component%20Object%20Reference) (OtherBodyIndex :type Integer) (bFromSweep :type Boolean) (SweepResult :type Hit%20Result%20Structure%20%28by%20ref%29))
  (Utilities|Casting|CastToBP_ThirdPersonCharacter OtherActor)
  (UserInterface|Viewport|AddtoViewport (Variables|Default|GetWInneract) 0))

(event Custom|Start%20Dialogue
  (bind _outrownames (DataTable|GetDataTableRowNames "/Game/DataTables/DT_Dialogue.DT_Dialogue"))
  (bind _returnvalue (Utilities|GetDataTableRow "/Game/DataTables/DT_Dialogue.DT_Dialogue" (Utilities|Array|Get(acopy) _outrownames (Variables|Default|GetRow%20Index)))
    (:then
      (Rendering|Components|TextRender|SetText (Variables|/Game/Blueprints/W_DialogueSystem.W_DialogueSystem_C|GetTextBlock_0 (Variables|Default|GetWDialogue)) (.text _returnvalue))
      (CallFunction|Picture)
      (Math|Integer|IncrementInt (Variables|Default|GetRow%20Index)))
    (:RowNotFound
      (Development|PrintString "BAD" true true "(R=0.000000,G=0.660000,B=1.000000,A=1.000000)" 8.0))))

(event Custom|Picture
  (bind _wdialogue (Variables|Default|GetWDialogue))
  (bind _image_0 (Variables|/Game/Blueprints/W_DialogueSystem.W_DialogueSystem_C|GetImage_0 _wdialogue))
  (switch Utilities|FlowControl|Switch|SwitchonE_Emotion (.emotion (stale Custom|Start%20Dialogue _returnvalue))
    (:NewEnumerator0
      (Class|Image|SetBrushfromMaterial _image_0 "/Game/Materials/GD2N_Mat.GD2N_Mat"))
    (:NewEnumerator1
      (Class|Image|SetBrushfromMaterial _image_0 "/Game/Materials/GD2Q_Mat.GD2Q_Mat"))
    (:NewEnumerator2
      (Class|Image|SetBrushfromMaterial _image_0 "/Game/Materials/GD2S_Mat.GD2S_Mat"))))

(event Custom|E_Pressed
  (UserInterface|Viewport|AddtoViewport (Variables|Default|GetWDialogue) 0)
  (CallFunction|StartDialogue))

(event EventBeginPlay
  (bind _returnvalue (UserInterface|CreateWidget "/Game/Blueprints/W_DialogueSystem.W_DialogueSystem_C"))
  (Variables|Default|SetWDialogue _returnvalue)
  (bind _returnvalue_2 (UserInterface|CreateWidget "/Game/Blueprints/W_Inneract.W_Inneract_C"))
  (Variables|Default|SetWInneract _returnvalue_2))

(fn ConstructionScript)