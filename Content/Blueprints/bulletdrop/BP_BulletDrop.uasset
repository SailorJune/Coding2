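; BP_BulletDrop is a debug Blueprint that simulates bullet drop from an Arrow component alongside the engine's projectile path prediction.
; BeginPlay starts an endless loop that draws the PredictProjectilePathAdvanced path, waits briefly, then runs a custom calculator.
; The calculator steps SimFrequency line traces, dividing only X velocity by frequency and adding per-step gravity to Z.
; It draws each segment, stops on a hit, then resets location and velocity.
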(event Custom|Really%20Cool%20Bullet%20Drop%20Calculator
  (bind _maxsimtime (Variables|Default|GetMaxSimTime))
  (Variables|Default|SetEnd (+ (Variables|Default|GetStart%20Location) (/ (Variables|Default|GetVelocity) (Math|Vector|MakeVector (Variables|Default|GetSim%20Frequency) 1.0 1.0))))
  (Utilities|FlowControl|ForLoopwithBreak 1 (Math|Float|Truncate (Variables|Default|GetSim%20Frequency)) :!label _label
    (:LoopBody
      (Rendering|Debug|DrawDebugLine (Variables|Default|GetStart%20Location) (Variables|Default|GetEnd) "(R=1.000000,G=0.072170,B=0.835632,A=1.000000)" _maxsimtime 0.0)
      (Rendering|Debug|DrawDebugSphere (Variables|Default|GetEnd) 5.0 12 "(R=0.000000,G=1.000000,B=0.992173,A=1.000000)" _maxsimtime)
      (bind _returnvalue (Class|KismetSystemLibrary|LineTraceSinglebyProfile (Variables|Default|GetStart%20Location) (Variables|Default|GetEnd) "BlockAll" false 0 "ForDuration" true))
      (if _returnvalue
        (Development|PrintString "HIT")
        (goto _label Break)
        (else
          (Variables|Default|SetStart%20Location (Variables|Default|GetEnd))
          (Variables|Default|SetVelocity (+ (Variables|Default|GetVelocity) (Math|Vector|MakeVector 0.0 0.0 (/ -9.8e+02 (Math|Float|Square (Variables|Default|GetSim%20Frequency))))))
          (Variables|Default|SetEnd (+ (Variables|Default|GetStart%20Location) (/ (Variables|Default|GetVelocity) (Math|Vector|MakeVector (Variables|Default|GetSim%20Frequency) 1.0 1.0)))))))
    (:Completed
      (Variables|Default|SetStart%20Location (Transformation|GetWorldLocation (Variables|Default|GetArrow)))
      (Variables|Default|SetVelocity (Variables|Default|GetStartingVelocity)))))

(event EventBeginPlay
  (Variables|Default|SetStart%20Location (Transformation|GetWorldLocation (Variables|Default|GetArrow)))
  (Class|GameplayStatics|BlueprintPredictProjectilePathAdvanced (Utilities|Struct|MakePredictProjectilePathParams (Variables|Default|GetStart%20Location) (Variables|Default|GetStartingVelocity) true 0.0 (Variables|Default|GetMaxSimTime) true "ECC_WorldStatic" "ObjectTypeQuery1" 0 (Variables|Default|GetSim%20Frequency) 0.0 "ForDuration" 1.0 false) :!label _label)
  (Utilities|FlowControl|Delay 1.5)
  (Utilities|FlowControl|Sequence
    (:then_0
      (CallFunction|ReallyCoolBulletDropCalculator))
    (:then_1
      (goto _label))))

(fn ConstructionScript)