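; BP_Weapon is a weapon Blueprint with a type, an element and a damage range, all shown on text components.
; SetMesh applies the weapon mesh to WeaponBody and picks its material from the element: Fire, Ice, Candy or Slime.
; randomizevalues randomly bumps minimum damage, derives maximum from it, then calls UpdateText to refresh the type, element and damage labels.
; The construction script is empty, and nothing here calls SetMesh or randomizevalues.
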(event Custom|SetMesh
  (Components|StaticMesh|SetStaticMesh (Variables|Default|GetWeapon%20Body) (Variables|Default|GetWeapon%20Mesh))
  (switch Utilities|FlowControl|Switch|SwitchonE_DamageType (Variables|Default|GetElmType)
    (:NewEnumerator1
      (Rendering|Material|SetMaterial (Variables|Default|GetWeapon%20Body) 0 "/AnimationSharing/AnimSharingRed.AnimSharingRed"))
    (:NewEnumerator2
      (Rendering|Material|SetMaterial (Variables|Default|GetWeapon%20Body) 0 "/AnimationSharing/AnimSharingBlue.AnimSharingBlue"))
    (:NewEnumerator3
      (Rendering|Material|SetMaterial (Variables|Default|GetWeapon%20Body) 0 "/DatasmithContent/Materials/AliasReference.AliasReference"))
    (:NewEnumerator4
      (Rendering|Material|SetMaterial (Variables|Default|GetWeapon%20Body) 0 "/AnimationSharing/AnimSharingGreen.AnimSharingGreen"))))

(event Custom|randomize%20values
  (bind _output_get (Variables|Default|SetMinDmg (+ (Variables|Default|GetMinDmg) (Math|Random|RandomInteger 2))))
  (Variables|Default|SetMaxDmg (+ _output_get (Math|Random|RandomIntegerinRange 1 4)))
  (CallFunction|UpdateText))

(event Custom|UpdateText
  (Rendering|Components|TextRender|SetText (Variables|Default|GetTextWpnTyp) (Utilities|Text|ToText(String) (Utilities|String|EnumtoString (Variables|Default|GetWpnType))))
  (Rendering|Components|TextRender|SetText (Variables|Default|GetTextDmgTyp) (Utilities|Text|ToText(String) (Utilities|String|EnumtoString (Variables|Default|GetElmType))))
  (Rendering|Components|TextRender|SetText (Variables|Default|GetTextDmg) (Utilities|Text|ToText(String) (Utilities|String|Append (Utilities|String|ToString(Integer) (Variables|Default|GetMinDmg)) "-" (Utilities|String|ToString(Integer) (Variables|Default|GetMaxDmg))))))

(fn ConstructionScript)