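; BP_DeleteLevelSaves is a trigger actor that opens a save-deletion menu when the third-person character walks into its box.
; On BeginPlay it creates the NewWidgetBlueprint widget and stores it.
; On box overlap by BP_ThirdPersonCharacter it stops the character's movement, adds the widget to the viewport, shows the mouse cursor and switches input to UI only.
; The deletion itself is not handled in this actor.
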(event OnComponentBeginOverlap(Box)
  (params (OverlappedComponent :type Primitive%20Component%20Object%20Reference) (OtherActor :type Actor%20Object%20Reference) (OtherComp :type Primitive%20Component%20Object%20Reference) (OtherBodyIndex :type Integer) (bFromSweep :type Boolean) (SweepResult :type Hit%20Result%20Structure%20%28by%20ref%29))
  (bind _returnvalue (Game|GetPlayerController 0))
  (bind _asbp_third_person_character (Utilities|Casting|CastToBP_ThirdPersonCharacter OtherActor))
  (Components|Movement|StopMovementImmediately (Variables|/Script/Engine.Character|GetCharacterMovement _asbp_third_person_character))
  (UserInterface|Viewport|AddtoViewport (Variables|Default|GetDeleteSavesWidget) 0)
  (Variables|/Script/Engine.PlayerController|SetbShowMouseCursor _returnvalue true)
  (Input|SetInputModeUIOnly _returnvalue 0 "DoNotLock" false))

(event EventBeginPlay
  (bind _returnvalue (UserInterface|CreateWidget "/Game/WidgetsUI/NewWidgetBlueprint.NewWidgetBlueprint_C"))
  (Variables|Default|SetDeleteSavesWidget _returnvalue))

(event Collision|EventActorBeginOverlap
  (params (OtherActor :type Actor%20Object%20Reference)))

(event EventTick
  (params (DeltaSeconds :type Float%20%28single-precision%29)))

(fn ConstructionScript)