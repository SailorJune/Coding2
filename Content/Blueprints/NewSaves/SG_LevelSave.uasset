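; SG_LevelSave is a level save Blueprint that restores the state of collected coins, with an unfinished counterpart for opened doors.
; LoadCollectedCoins loops over the CollectedCoins array and calls LoadCollectedState on each valid entry.
; LoadOpenedDoors is a stub that iterates the same CollectedCoins array instead of a door list and does nothing with valid entries.
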(fn LoadCollectedCoins
  (if (> (Utilities|Array|Length (Variables|Default|GetCollectedCoins)) 0)
    (for _array_element (Variables|Default|GetCollectedCoins)
      (Utilities|IsValid _array_element
        (:Is%20Valid
          (Default|LoadCollectedState _array_element))))))

(fn LoadOpenedDoors
  (if (> (Utilities|Array|Length (Variables|Default|GetCollectedCoins)) 0)
    (for _array_element (Variables|Default|GetCollectedCoins)
      (Utilities|IsValid _array_element))))