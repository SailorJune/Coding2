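; Split-screen game mode that manages per-level saves, checkpoints and extra local players.
; BeginPlay loads the save slot named after the level to restore coins, doors and weapons, or creates one if none exists.
; A non-zero saved position teleports the first player there and spawns additional players based on NumPlayers.
; Checkpoint saves a transform, LevelEnd clears it, and Win quits once both winning flags are set.
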(event Custom|Save%20Game
  (bind _returnvalue (Game|GetCurrentLevelName true))
  (bind _returnvalue_2 (SaveGame|SaveGametoSlot (Variables|Default|GetLevel%20Save) _returnvalue))
  (if _returnvalue_2
    (Development|PrintString "Saved Level")
    (else
      (Development|PrintString "Didn't save level"))))

(event Custom|Win
  (if (Variables|Default|GetWinning1)
    (if (Variables|Default|GetWinning%202)
      (Game|QuitGame 0 "Quit" false))))

(event EventBeginPlay
  (Development|PrintString "Loaded into the GM_Coding2ForReal Game Mode" true true "(R=0.481250,G=0.000000,B=0.001624,A=1.000000)")
  (bind _returnvalue (Game|GetCurrentLevelName true))
  (bind _returnvalue_2 (SaveGame|DoesSaveGameExist _returnvalue))
  (if _returnvalue_2
    (bind _returnvalue_3 (SaveGame|LoadGamefromSlot _returnvalue))
    (bind _assg_level_save (Utilities|Casting|CastToSG_LevelSave _returnvalue_3)
      (:then
        (bind _output_get (Variables|Default|SetLevel%20Save _assg_level_save))
        (Default|LoadCollectedCoins _output_get)
        (Default|LoadOpenedDoors (Variables|Default|GetLevel%20Save))
        (Default|LoadSpawnedWeapons (Variables|Default|GetLevel%20Save))
        (if (not (Class|KismetMathLibrary|EqualExactlyVectorVector (.location (Variables|/Game/Blueprints/NewSaves/SG_LevelSave.SG_LevelSave_C|GetPlayerTransform (Variables|Default|GetLevel%20Save))) "0, 0, 0"))
          (Transformation|SetWorldTransform (Variables|/Script/Engine.Character|GetCapsuleComponent (Game|GetPlayerCharacter 0)) (Variables|/Game/Blueprints/NewSaves/SG_LevelSave.SG_LevelSave_C|GetPlayerTransform (Variables|Default|GetLevel%20Save)) false false)
          (Utilities|FlowControl|Sequence
            (:then_0
              (switch Utilities|FlowControl|Switch|SwitchonE_Players (Variables|Default|GetNumPlayers)
                (:NewEnumerator1
                  (goto _label Reset))
                (:NewEnumerator2
                  (Utilities|FlowControl|Sequence
                    (:then_0
                      (goto _label Reset))
                    (:then_1
                      (goto _label_2 Reset))))))
            (:then_1
              (Class|GameplayStatics|CreatePlayer 1)
              (Utilities|FlowControl|DoOnce true :!label _label
                (:Completed
                  (Class|GameplayStatics|CreatePlayer 2)
                  (Utilities|FlowControl|DoOnce false :!label _label_2
                    (:Completed
                      (Class|GameplayStatics|CreatePlayer 3)))))))))
      (:CastFailed
        (SaveGame|DeleteGameinSlot _returnvalue)))
    (else
      (bind _returnvalue_4 (SaveGame|CreateSaveGameObject "/Game/Blueprints/NewSaves/SG_LevelSave.SG_LevelSave_C"))
      (Variables|Default|SetLevel%20Save _returnvalue_4))))

(fn ConstructionScript)

(fn Checkpoint
  (params (Player%20Transform :type Transform))
  (Variables|/Game/Blueprints/NewSaves/SG_LevelSave.SG_LevelSave_C|SetPlayerTransform (Variables|Default|GetLevel%20Save) Player%20Transform)
  (CallFunction|SaveGame))

(fn LevelEnd
  (Variables|/Game/Blueprints/NewSaves/SG_LevelSave.SG_LevelSave_C|SetPlayerTransform (Variables|Default|GetLevel%20Save) "")
  (CallFunction|SaveGame))