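; BP_Maze2 is a split-screen maze actor whose Cube rotates in 90-degree yaw steps.
; TurnRight and TurnLeft events each lerp the rotation through their own Timeline, holding a Turning flag until it finishes.
; A Box trigger sets InRange2 on an overlapping BP_ThirdPersonSS and shows a button prompt widget created at BeginPlay, reversing both on exit.
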(event OnComponentBeginOverlap(Box)
  (params (OverlappedComponent :type Primitive%20Component%20Object%20Reference) (OtherActor :type Actor%20Object%20Reference) (OtherComp :type Primitive%20Component%20Object%20Reference) (OtherBodyIndex :type Integer) (bFromSweep :type Boolean) (SweepResult :type Hit%20Result%20Structure%20%28by%20ref%29))
  (bind _asbp_third_person_ss (Utilities|Casting|CastToBP_ThirdPersonSS OtherActor))
  (Variables|/Game/Blueprints/Splitscreen/BP_ThirdPersonSS.BP_ThirdPersonSS_C|SetInRange2 _asbp_third_person_ss true)
  (UserInterface|Viewport|AddtoViewport (Variables|Default|GetWidget) 0))

(event OnComponentEndOverlap(Box)
  (params (OverlappedComponent :type Primitive%20Component%20Object%20Reference) (OtherActor :type Actor%20Object%20Reference) (OtherComp :type Primitive%20Component%20Object%20Reference) (OtherBodyIndex :type Integer))
  (bind _asbp_third_person_ss (Utilities|Casting|CastToBP_ThirdPersonSS OtherActor))
  (Variables|/Game/Blueprints/Splitscreen/BP_ThirdPersonSS.BP_ThirdPersonSS_C|SetInRange2 _asbp_third_person_ss false)
  (Widget|RemovefromParent (Variables|Default|GetWidget)))

(event Custom|Turn%20Right
  (bind _cube (Variables|Default|GetCube))
  (bind _relativerotation (Variables|/Script/Engine.SceneComponent|GetRelativeRotation _cube))
  (Development|PrintString "turning")
  (Variables|Default|SetTurning? true)
  (Variables|Default|SetEndRotation (+ (.yaw _relativerotation) 9e+01))
  (Variables|Default|SetStartRotation (.yaw _relativerotation))
  (bind _newtrack_0 (Timeline|Timeline PlayFromStart)
    (:Update
      (Transformation|SetRelativeRotation _cube (Math|Rotator|Lerp(Rotator) (Math|Rotator|MakeRotator 0.0 0.0 (Variables|Default|GetStartRotation)) (Math|Rotator|MakeRotator 0.0 0.0 (Variables|Default|GetEndRotation)) _newtrack_0) false false))
    (:Finished
      (Variables|Default|SetTurning? false))))

(event Custom|Turn%20Left
  (bind _cube (Variables|Default|GetCube))
  (bind _relativerotation (Variables|/Script/Engine.SceneComponent|GetRelativeRotation _cube))
  (Development|PrintString "Turning Left")
  (Variables|Default|SetTurning? true)
  (Variables|Default|SetStartRotation (.yaw _relativerotation))
  (Variables|Default|SetEndRotation (- (.yaw _relativerotation) 9e+01))
  (bind _newtrack_0 (Timeline|Timeline_0 PlayFromStart)
    (:Update
      (Transformation|SetRelativeRotation _cube (Math|Rotator|Lerp(Rotator) (Math|Rotator|MakeRotator 0.0 0.0 (Variables|Default|GetStartRotation)) (Math|Rotator|MakeRotator 0.0 0.0 (Variables|Default|GetEndRotation)) _newtrack_0) false false))
    (:Finished
      (Variables|Default|SetTurning? false))))

(event EventBeginPlay
  (bind _returnvalue (UserInterface|CreateWidget "/Game/Blueprints/Splitscreen/W_ButtonPrompt1.W_ButtonPrompt1_C"))
  (Variables|Default|SetWidget _returnvalue))

(fn ConstructionScript)