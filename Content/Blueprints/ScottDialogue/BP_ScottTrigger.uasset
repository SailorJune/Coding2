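; Trigger Blueprint that shows Scott and Ramona dialogue when the player character overlaps its box.
; It creates the W_Scott widget shortly after BeginPlay, then on overlap halts the character's movement and adds the widget to the viewport.
; StartDialogue displays the DT_Scott row at RowIndex and increments the index, so each call shows one line.
; Picture maps that row's Speaker value to a portrait material on the widget's image.
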(event OnComponentBeginOverlap(Box)
  (params (OverlappedComponent :type Primitive%20Component%20Object%20Reference) (OtherActor :type Actor%20Object%20Reference) (OtherComp :type Primitive%20Component%20Object%20Reference) (OtherBodyIndex :type Integer) (bFromSweep :type Boolean) (SweepResult :type Hit%20Result%20Structure%20%28by%20ref%29))
  (bind _asbp_third_person_character (Utilities|Casting|CastToBP_ThirdPersonCharacter OtherActor))
  (Components|Movement|StopMovementImmediately (Variables|/Script/Engine.Character|GetCharacterMovement _asbp_third_person_character))
  (UserInterface|Viewport|AddtoViewport (Variables|Default|GetScottWidget) 0)
  (CallFunction|StartDialogue))

(event Custom|StartDialogue
  (Development|PrintString "Starting Dialoge")
  (bind _outrownames (DataTable|GetDataTableRowNames "/Game/Blueprints/ScottDialogue/DT_Scott.DT_Scott"))
  (bind _returnvalue (Utilities|GetDataTableRow "/Game/Blueprints/ScottDialogue/DT_Scott.DT_Scott" (Utilities|Array|Get(acopy) _outrownames (Variables|Default|GetRowIndex)))
    (:then
      (Rendering|Components|TextRender|SetText (Variables|/Game/Blueprints/ScottDialogue/W_Scott.W_Scott_C|GetTextBlock_0 (Variables|Default|GetScottWidget)) (.text _returnvalue))
      (CallFunction|Picture)
      (Math|Integer|IncrementInt (Variables|Default|GetRowIndex)))
    (:RowNotFound
      (Development|PrintString "Row not found :("))))

(event Custom|Picture
  (bind _scottwidget (Variables|Default|GetScottWidget))
  (bind _image_0 (Variables|/Game/Blueprints/ScottDialogue/W_Scott.W_Scott_C|GetImage_0 _scottwidget))
  (switch Utilities|FlowControl|Switch|SwitchonE_Character (.speaker (stale Custom|StartDialogue _returnvalue))
    (:NewEnumerator0
      (Class|Image|SetBrushfromMaterial _image_0 "/Game/Blueprints/ScottDialogue/M_ScottHappy.M_ScottHappy"))
    (:NewEnumerator1
      (Class|Image|SetBrushfromMaterial _image_0 "/Game/Blueprints/ScottDialogue/M_Scottnervous.M_Scottnervous"))
    (:NewEnumerator2
      (Class|Image|SetBrushfromMaterial _image_0 "/Game/Blueprints/ScottDialogue/M_ScottSad.M_ScottSad"))
    (:NewEnumerator3
      (Class|Image|SetBrushfromMaterial _image_0 "/Game/Blueprints/ScottDialogue/M_RamonaNeutral.M_RamonaNeutral"))
    (:NewEnumerator4
      (Class|Image|SetBrushfromMaterial _image_0 "/Game/Blueprints/ScottDialogue/M_RamonaAnnoyed.M_RamonaAnnoyed"))))

(event EventBeginPlay
  (Utilities|FlowControl|Delay 2.0)
  (bind _returnvalue (UserInterface|CreateWidget "/Game/Blueprints/ScottDialogue/W_Scott.W_Scott_C"))
  (Variables|Default|SetScottWidget _returnvalue))

(fn ConstructionScript)