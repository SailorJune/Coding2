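; BP_DiaTrigger is a box trigger that plays one dialogue line each time the third-person character overlaps it, halting the character's current movement.
; It shows a W_ScottWidget created shortly after BeginPlay and reads the next DT_DialogueFinal row by an incrementing index.
; Each row sets the text, plays its voice clip and swaps the image material by Speaker value.
; A failed row lookup removes the widget.
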(event OnComponentBeginOverlap(Box)
  (params (OverlappedComponent :type Primitive%20Component%20Object%20Reference) (OtherActor :type Actor%20Object%20Reference) (OtherComp :type Primitive%20Component%20Object%20Reference) (OtherBodyIndex :type Integer) (bFromSweep :type Boolean) (SweepResult :type Hit%20Result%20Structure%20%28by%20ref%29))
  (bind _asbp_third_person_character (Utilities|Casting|CastToBP_ThirdPersonCharacter OtherActor))
  (Components|Movement|StopMovementImmediately (Variables|/Script/Engine.Character|GetCharacterMovement _asbp_third_person_character))
  (UserInterface|Viewport|AddtoViewport (Variables|Default|GetDiaWidget) 0)
  (CallFunction|StartDialogue))

(event Custom|StartDialogue
  (Development|PrintString "Starting Dialoge")
  (bind _outrownames (DataTable|GetDataTableRowNames "/Game/Blueprints/FinalDialogue/DT_DialogueFinal.DT_DialogueFinal"))
  (bind _returnvalue (Utilities|GetDataTableRow "/Game/Blueprints/FinalDialogue/DT_DialogueFinal.DT_DialogueFinal" (Utilities|Array|Get(acopy) _outrownames (Variables|Default|GetRowIndex)))
    (:then
      (Rendering|Components|TextRender|SetText (Variables|/Game/Blueprints/FinalDialogue/W_ScottWidget.W_ScottWidget_C|GetTextBlock_0 (Variables|Default|GetDiaWidget)) (.text _returnvalue))
      (Audio|PlaySound2D (.spokentext _returnvalue) 1.0 1.0 0.0 0 0)
      (CallFunction|Picture)
      (Math|Integer|IncrementInt (Variables|Default|GetRowIndex)))
    (:RowNotFound
      (Widget|RemovefromParent (Variables|Default|GetDiaWidget)))))

(event Custom|Picture
  (bind _diawidget (Variables|Default|GetDiaWidget))
  (bind _image_68 (Variables|/Game/Blueprints/FinalDialogue/W_ScottWidget.W_ScottWidget_C|GetImage_68 _diawidget))
  (switch Utilities|FlowControl|Switch|SwitchonE_Character (.speaker (stale Custom|StartDialogue _returnvalue))
    (:NewEnumerator0
      (Class|Image|SetBrushfromMaterial _image_68 "/Game/Blueprints/FinalDialogue/M_Point.M_Point"))
    (:NewEnumerator1
      (Class|Image|SetBrushfromMaterial _image_68 "/Game/Blueprints/FinalDialogue/M_ThumbsUP.M_ThumbsUP"))
    (:NewEnumerator2
      (Class|Image|SetBrushfromMaterial _image_68 "/Game/Blueprints/FinalDialogue/M_Book.M_Book"))
    (:NewEnumerator3
      (Class|Image|SetBrushfromMaterial _image_68 "/Game/Blueprints/FinalDialogue/M_Fridge.M_Fridge"))
    (:NewEnumerator4
      (Class|Image|SetBrushfromMaterial _image_68 "/Game/Blueprints/FinalDialogue/M_Cool.M_Cool"))))

(event EventBeginPlay
  (Utilities|FlowControl|Delay 2.0)
  (bind _returnvalue (UserInterface|CreateWidget "/Game/Blueprints/FinalDialogue/W_ScottWidget.W_ScottWidget_C"))
  (Variables|Default|SetDiaWidget _returnvalue))

(fn ConstructionScript)