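; SG_SaveLoad is a Game Instance that saves, loads and deletes player and level progress.
; Player stamina, transform and sprint/shoot flags pass between BP_ThirdPersonCharacter and a GI_PlayerSAve slot.
; Level state lives in SG_LevelSave, cached on Init under a slot named after the current level, and loading reapplies its collected objects.
; Save and Load run both halves, while deletion removes both slots, clears collected objects and reopens the level.
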(event Custom|SaveGame
  ;[1 1 1] Saving Player Details
  (Development|PrintString "Starting Save Game")
  (bind _returnvalue (SaveGame|DoesSaveGameExist (Variables|Default|GetSlot%20Name)))
  (if _returnvalue
    (bind _returnvalue_2 (SaveGame|LoadGamefromSlot (Variables|Default|GetSlot%20Name)))
    (Variables|Default|SetSaverSubclass _returnvalue_2)
    (else
      (bind _returnvalue_3 (SaveGame|CreateSaveGameObject "/Game/Blueprints/GI_PlayerSAve.GI_PlayerSAve_C"))
      (Variables|Default|SetSaverSubclass _returnvalue_3)))
  (bind _asgi_player_save (Utilities|Casting|CastToGI_PlayerSAve (Variables|Default|GetSaverSubclass)))
  (bind _asbp_third_person_character (Utilities|Casting|CastToBP_ThirdPersonCharacter (Game|GetPlayerCharacter 0)))
  (Variables|/Game/Blueprints/GI_PlayerSAve.GI_PlayerSAve_C|SetPlayerStamina _asgi_player_save (Variables|/Game/ThirdPerson/Blueprints/BP_ThirdPersonCharacter.BP_ThirdPersonCharacter_C|GetStamina _asbp_third_person_character))
  (Variables|/Game/Blueprints/GI_PlayerSAve.GI_PlayerSAve_C|SetPlayerTransform _asgi_player_save (Transformation|GetWorldTransform (Variables|/Script/Engine.Character|GetCapsuleComponent _asbp_third_person_character)))
  (Variables|/Game/Blueprints/GI_PlayerSAve.GI_PlayerSAve_C|SetPlayerCanSprint _asgi_player_save (Variables|/Game/ThirdPerson/Blueprints/BP_ThirdPersonCharacter.BP_ThirdPersonCharacter_C|GetCanSprint _asbp_third_person_character))
  (Variables|/Game/Blueprints/GI_PlayerSAve.GI_PlayerSAve_C|SetPlayerCanShoot _asgi_player_save (Variables|/Game/ThirdPerson/Blueprints/BP_ThirdPersonCharacter.BP_ThirdPersonCharacter_C|GetCanShoot _asbp_third_person_character))
  (Development|PrintString "Game is currently saved")
  (SaveGame|SaveGametoSlot _asgi_player_save (Variables|Default|GetSlot%20Name)))

(event Custom|LoadGame
  ;[1 1 1] Saving Player Details
  (Development|PrintString "Starting Load Game")
  (bind _returnvalue (SaveGame|DoesSaveGameExist (Variables|Default|GetSlot%20Name)))
  (if _returnvalue
    (bind _returnvalue_2 (SaveGame|LoadGamefromSlot (Variables|Default|GetSlot%20Name)))
    (bind _output_get (Variables|Default|SetSaverSubclass _returnvalue_2))
    (bind _asgi_player_save (Utilities|Casting|CastToGI_PlayerSAve _output_get))
    (bind _asbp_third_person_character (Utilities|Casting|CastToBP_ThirdPersonCharacter (Game|GetPlayerCharacter 0)))
    (Variables|/Game/ThirdPerson/Blueprints/BP_ThirdPersonCharacter.BP_ThirdPersonCharacter_C|SetStamina _asbp_third_person_character (Variables|/Game/Blueprints/GI_PlayerSAve.GI_PlayerSAve_C|GetPlayerStamina _asgi_player_save))
    (Transformation|SetWorldTransform (Variables|/Script/Engine.Character|GetCapsuleComponent _asbp_third_person_character) (Variables|/Game/Blueprints/GI_PlayerSAve.GI_PlayerSAve_C|GetPlayerTransform _asgi_player_save) false false)
    (Variables|/Game/ThirdPerson/Blueprints/BP_ThirdPersonCharacter.BP_ThirdPersonCharacter_C|SetCanShoot _asbp_third_person_character (Variables|/Game/Blueprints/GI_PlayerSAve.GI_PlayerSAve_C|GetPlayerCanShoot _asgi_player_save))
    (Variables|/Game/ThirdPerson/Blueprints/BP_ThirdPersonCharacter.BP_ThirdPersonCharacter_C|SetCanSprint _asbp_third_person_character (Variables|/Game/Blueprints/GI_PlayerSAve.GI_PlayerSAve_C|GetPlayerCanSprint _asgi_player_save))
    (Development|PrintString "Game Loaded")))

(event Custom|SaveLevel
  (Development|PrintString "Saving Level from game instance" true true "(R=0.906868,G=0.000000,B=1.000000,A=1.000000)")
  (bind _returnvalue (Game|GetCurrentLevelName true))
  (bind _returnvalue_2 (SaveGame|SaveGametoSlot (Variables|Default|GetLevel%20Data) _returnvalue))
  (if _returnvalue_2
    (Development|PrintString "level saved")
    (else
      (Development|PrintString "Boowomp"))))

(event Custom|LoadLevel
  (Development|PrintString "Loading Level From Game Instance" true true "(R=0.888690,G=0.000000,B=1.000000,A=1.000000)")
  (bind _returnvalue (Game|GetCurrentLevelName true))
  (bind _returnvalue_2 (SaveGame|DoesSaveGameExist _returnvalue))
  (if _returnvalue_2
    (bind _returnvalue_3 (SaveGame|LoadGamefromSlot _returnvalue))
    (bind _output_get (Variables|Default|SetSaverSubclass _returnvalue_3))
    (bind _assg_level_save (Utilities|Casting|CastToSG_LevelSave _output_get))
    (bind _output_get_2 (Variables|Default|SetLevel%20Data _assg_level_save))
    (Default|LoadCollectedObjects _output_get_2)
    (Development|PrintString "loaded objects")
    (else
      (Development|PrintString "Save doesn't exist"))))

(event Custom|Save
  (CallFunction|SaveGame)
  (CallFunction|SaveLevel))

(event Custom|Load
  (CallFunction|LoadGame)
  (CallFunction|LoadLevel))

(event Custom|DeleteSaveData
  (Development|PrintString "de")
  (bind _returnvalue (SaveGame|DeleteGameinSlot (Variables|Default|GetSlot%20Name)))
  (if _returnvalue
    (bind _returnvalue_2 (Game|GetCurrentLevelName true))
    (bind _returnvalue_3 (SaveGame|DeleteGameinSlot _returnvalue_2))
    (if _returnvalue_3
      (Utilities|Array|Clear (Variables|/Game/Blueprints/SG_LevelSave.SG_LevelSave_C|GetCollectedObjects (Variables|Default|GetLevel%20Data)))
      (Development|PrintString "Save Data Deleted")
      (bind _returnvalue_4 (Game|GetCurrentLevelName true))
      (Game|OpenLevel(byName) (Utilities|String|StringToName _returnvalue_4))
      (else
        (Development|PrintString "te")))
    (else
      (Development|PrintString "le"))))

(event EventInit
  (bind _returnvalue (Game|GetCurrentLevelName true))
  (bind _returnvalue_2 (SaveGame|DoesSaveGameExist _returnvalue))
  (if _returnvalue_2
    (bind _returnvalue_3 (SaveGame|LoadGamefromSlot _returnvalue))
    (bind _assg_level_save (Utilities|Casting|CastToSG_LevelSave _returnvalue_3))
    (Variables|Default|SetLevel%20Data _assg_level_save)
    (else
      (bind _returnvalue_4 (SaveGame|CreateSaveGameObject "/Game/Blueprints/SG_LevelSave.SG_LevelSave_C"))
      (Variables|Default|SetLevel%20Data _returnvalue_4))))