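; Game Instance that saves, loads and deletes player and per-level progress.
; Player stamina, transform and shoot/sprint flags go into SG_PlayerSave under SlotName, while SG_LevelSave uses the current level name as its slot.
; Init loads or creates the cached LevelData, which SaveLevel writes and LoadLevel reloads to call LoadCollectedObjects.
; SaveAll and LoadAll combine both saves, and DeleteSaveData removes both slots and reopens the level.
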(event Custom|Save%20Game
  ;[1 1 1] Save
  (Development|PrintString "Starting Save Game")
  (bind _returnvalue (SaveGame|DoesSaveGameExist (Variables|Default|GetSlot%20Name)))
  (if _returnvalue
    (bind _returnvalue_2 (SaveGame|LoadGamefromSlot (Variables|Default|GetSlot%20Name)))
    (Variables|Default|SetSaver%20Subclass _returnvalue_2)
    (else
      (bind _returnvalue_3 (SaveGame|CreateSaveGameObject "/Game/Blueprints/SG_PlayerSave.SG_PlayerSave_C"))
      (Variables|Default|SetSaver%20Subclass _returnvalue_3)))
  (bind _assg_player_save (Utilities|Casting|CastToSG_PlayerSave (Variables|Default|GetSaver%20Subclass)))
  (bind _asbp_third_person_character (Utilities|Casting|CastToBP_ThirdPersonCharacter (Game|GetPlayerCharacter 0)))
  (Variables|/Game/Blueprints/SG_PlayerSave.SG_PlayerSave_C|SetPlayer%20Stamina _assg_player_save (Variables|/Game/ThirdPerson/Blueprints/BP_ThirdPersonCharacter.BP_ThirdPersonCharacter_C|GetStamina _asbp_third_person_character))
  (Variables|/Game/Blueprints/SG_PlayerSave.SG_PlayerSave_C|SetPlayer%20Transform _assg_player_save (Transformation|GetWorldTransform (Variables|/Script/Engine.Character|GetCapsuleComponent _asbp_third_person_character)))
  (Variables|/Game/Blueprints/SG_PlayerSave.SG_PlayerSave_C|SetPlayerCanShoot _assg_player_save (Variables|/Game/ThirdPerson/Blueprints/BP_ThirdPersonCharacter.BP_ThirdPersonCharacter_C|GetCanShoot _asbp_third_person_character))
  (Variables|/Game/Blueprints/SG_PlayerSave.SG_PlayerSave_C|SetPlayerCanSprint _assg_player_save (Variables|/Game/ThirdPerson/Blueprints/BP_ThirdPersonCharacter.BP_ThirdPersonCharacter_C|GetCanSprint _asbp_third_person_character))
  (SaveGame|SaveGametoSlot _assg_player_save (Variables|Default|GetSlot%20Name))
  (Development|PrintString "Save Complete"))

(event Custom|Load%20Game
  ;[1 0.5344 0.5344] Load
  (Development|PrintString "Starting Game Load")
  (bind _returnvalue (SaveGame|DoesSaveGameExist (Variables|Default|GetSlot%20Name)))
  (if _returnvalue
    (bind _returnvalue_2 (SaveGame|LoadGamefromSlot (Variables|Default|GetSlot%20Name)))
    (bind _output_get (Variables|Default|SetSaver%20Subclass _returnvalue_2))
    (bind _assg_player_save (Utilities|Casting|CastToSG_PlayerSave _output_get))
    (bind _asbp_third_person_character (Utilities|Casting|CastToBP_ThirdPersonCharacter (Game|GetPlayerCharacter 0)))
    (Variables|/Game/ThirdPerson/Blueprints/BP_ThirdPersonCharacter.BP_ThirdPersonCharacter_C|SetStamina _asbp_third_person_character (Variables|/Game/Blueprints/SG_PlayerSave.SG_PlayerSave_C|GetPlayer%20Stamina _assg_player_save))
    (Variables|/Game/ThirdPerson/Blueprints/BP_ThirdPersonCharacter.BP_ThirdPersonCharacter_C|SetCanShoot _asbp_third_person_character (Variables|/Game/Blueprints/SG_PlayerSave.SG_PlayerSave_C|GetPlayerCanShoot _assg_player_save))
    (Variables|/Game/ThirdPerson/Blueprints/BP_ThirdPersonCharacter.BP_ThirdPersonCharacter_C|SetCanSprint _asbp_third_person_character (Variables|/Game/Blueprints/SG_PlayerSave.SG_PlayerSave_C|GetPlayerCanSprint _assg_player_save))
    (Transformation|SetActorTransform _asbp_third_person_character (Variables|/Game/Blueprints/SG_PlayerSave.SG_PlayerSave_C|GetPlayer%20Transform _assg_player_save))
    (SaveGame|LoadGamefromSlot (Variables|Default|GetSlot%20Name))))

(event Custom|SaveLevel
  (bind _returnvalue (Game|GetCurrentLevelName true))
  (SaveGame|SaveGametoSlot (Variables|Default|GetLevel%20Data) _returnvalue))

(event Custom|LoadLevel
  (Development|PrintString "Loading Game World")
  (bind _returnvalue (Game|GetCurrentLevelName true))
  (bind _returnvalue_2 (SaveGame|DoesSaveGameExist _returnvalue))
  (if _returnvalue_2
    (bind _returnvalue_3 (SaveGame|LoadGamefromSlot _returnvalue))
    (bind _output_get (Variables|Default|SetSaver%20Subclass _returnvalue_3))
    (bind _assg_level_save (Utilities|Casting|CastToSG_LevelSave _output_get))
    (bind _output_get_2 (Variables|Default|SetLevel%20Data _assg_level_save))
    (Default|LoadCollectedObjects _output_get_2)))

(event Custom|Save%20All
  (CallFunction|SaveGame)
  (CallFunction|SaveLevel))

(event Custom|Load%20All
  (CallFunction|LoadGame)
  (CallFunction|LoadLevel))

(event Custom|Delete%20Save%20Data
  (SaveGame|DeleteGameinSlot (Variables|Default|GetSlot%20Name))
  (if true
    (bind _returnvalue (Game|GetCurrentLevelName true))
    (bind _returnvalue_2 (SaveGame|DeleteGameinSlot _returnvalue))
    (if _returnvalue_2
      (Development|PrintString ":3 Dweeted")
      (bind _returnvalue_3 (Game|GetCurrentLevelName true))
      (Game|OpenLevel(byName) (Utilities|String|StringToName _returnvalue_3))
      (Utilities|Array|Clear (Variables|/Game/Blueprints/SG_LevelSave.SG_LevelSave_C|GetCollectableObject (Variables|Default|GetLevel%20Data)))
      (else
        (Development|PrintString "IT DOESN\"T WORK 2")))
    (else
      (Development|PrintString "IT DOESN\"T WORK"))))

(event EventInit
  (Development|PrintString "Saving Game World")
  (bind _returnvalue (Game|GetCurrentLevelName true))
  (bind _returnvalue_2 (SaveGame|DoesSaveGameExist _returnvalue))
  (if _returnvalue_2
    (bind _returnvalue_3 (SaveGame|LoadGamefromSlot _returnvalue))
    (bind _assg_level_save (Utilities|Casting|CastToSG_LevelSave _returnvalue_3))
    (Variables|Default|SetLevel%20Data _assg_level_save)
    (else
      (bind _returnvalue_4 (SaveGame|CreateSaveGameObject "/Game/Blueprints/SG_LevelSave.SG_LevelSave_C"))
      (Variables|Default|SetLevel%20Data _returnvalue_4))))