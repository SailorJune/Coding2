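; BP_Patrol_Route is a patrol route Blueprint that supplies world-space waypoints from a spline.
; GetPatrolPointLocation advances the index through IncrementPatrolPoint, then returns that spline point's location.
; IncrementPatrolPoint ping-pongs by flipping Direction when the index reaches the point count or zero, printing a debug "Hello" otherwise.
; The IncrementPatrolPointIndex event is an empty stub.
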(event Custom|Increment%20Patrol%20Point%20Index)

(event EventBeginPlay)

(fn ConstructionScript)

(fn GetPatrolPointLocation
  (CallFunction|IncrementPatrolPoint)
  (return (Spline|GetLocationatSplinePoint (Variables|Default|GetSpline) (Variables|Default|GetPatrolIndex) "World")))

(fn IncrementPatrolPoint
  (bind _output_get (Variables|Default|SetPatrolIndex (+ (Variables|Default|GetPatrolIndex) (Variables|Default|GetDirection))))
  (if (>= _output_get (Spline|GetNumberOfSplinePoints (Variables|Default|GetSpline)))
    (Variables|Default|SetDirection -1)
    (elif (<= (Variables|Default|GetPatrolIndex) 0)
      (Variables|Default|SetDirection 1)
      (else
        (Development|PrintString "Hello"))))
  (return _output_get))