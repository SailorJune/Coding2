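; BP_PatrolRoute is a patrol route that serves successive world-space waypoints from the points of a spline component.
; GetPatrolPointLocation first advances the patrol index by Direction, then returns that spline point's location, so each call moves the route forward.
; The index wraps to zero past the last point; otherwise, an index at or below zero sets Direction to forward.
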(event Custom|Increment%20Patrol%20Point%20Index
  (Variables|Default|SetPatrolIndex (+ (Variables|Default|GetPatrolIndex) (Variables|Default|GetDirection)))
  (if (>= (Variables|Default|GetPatrolIndex) (Spline|GetNumberOfSplinePoints (Variables|Default|GetSpline)))
    (Variables|Default|SetPatrolIndex 0)
    (elif (<= (Variables|Default|GetPatrolIndex) 0)
      (Variables|Default|SetDirection 1))))

(fn ConstructionScript)

(fn GetPatrolPointLocation
  (CallFunction|IncrementPatrolPointIndex)
  (return (Spline|GetLocationatSplinePoint (Variables|Default|GetSpline) (Variables|Default|GetPatrolIndex) "World")))